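; BP_Ai_Sub is a PaperZD character Blueprint with side-scrolling movement along the X axis and jumping, driven by input bindings.
; Jumping or walking off a ledge sends the PaperZD animation instance to its JumpActivated node, and landing clears the Jumping flag.
; Any damage received is only printed on screen as red debug text, with no health handling in this graph.
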(event `self.ReceiveAnyDamage`
  (params (Damage :type "Float (single-precision)") (DamageType :type "DamageType Object Reference") (InstigatedBy :type "Controller Object Reference") (DamageCauser :type "Actor Object Reference"))
  (`KismetSystemLibrary.PrintString` (`KismetStringLibrary.Concat_StrStr` "Taken Dame" (`KismetStringLibrary.Conv_DoubleToString` Damage)) true true (struct :`R` 0.693872 :`G` 0.027321 :`B` 0.027321 :`A` 1.0) 4.0))

(event `InputAxis|MoveRight`
  (params (AxisValue :type "Float (single-precision)"))
  (`self.AddMovementInput` (1.0 0.0 0.0) AxisValue))

(event `InputAction|Jump`
  (params (Key :type "Key Structure"))
  (:`Pressed`
    (`self.Jump`)))

(event `self.OnLanded`
  (params (Hit :type "HitResult Structure (by ref)"))
  (set `self.Jumping` false))

(event `self.OnJumped`
  (`PaperZDAnimInstance.JumpToNode` (`PaperZDAnimationComponent.AnimInstance` (`self.AnimationComponent`)) "JumpActivated" "None" :!label _label))

(event `self.OnWalkingOffLedge`
  (params (PreviousFloorImpactNormal :type "Vector Structure (by ref)") (PreviousFloorContactNormal :type "Vector Structure (by ref)") (PreviousLocation :type "Vector Structure (by ref)") (TimeDelta :type "Float (single-precision)"))
  (goto _label))

(fn `UserConstructionScript`)